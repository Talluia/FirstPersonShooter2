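; Player controller that shows the player's starting UI once the MAP2 level is active.
; Tick checks the level name and fires Show UI On Start through a DoOnce gate.
; That event casts the controlled pawn to FirstPersonCharacter and has it create chat, team selection and the user interface.
; A failed cast resets the gate, so the setup retries until the character is possessed.
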(event Custom|Show_UI_On_Start
  (bind _self self)
  (bind _asfirst_person_character (Utilities|Casting|CastToFirstPersonCharacter (Pawn|GetControlledPawn))
    (:then
      (Default|CreateChat _asfirst_person_character _self)
      (Default|ChooseTeams _asfirst_person_character _self)
      (Default|CreateUserInterface _asfirst_person_character))
    (:CastFailed
      (Utilities|FlowControl|DoOnce false) ; enters at Reset
    )))

(event EventBeginPlay)

(event EventTick
  (params (DeltaSeconds :type Float%20%28single-precision%29))
  (bind _returnvalue (Game|GetCurrentLevelName true))
  (if (Utilities|Enum|Equal(Enum) _returnvalue "MAP2")
    (Utilities|FlowControl|DoOnce false
      (:Completed
        (CallFunction|ShowUIonStart)))))

(fn ConstructionScript)